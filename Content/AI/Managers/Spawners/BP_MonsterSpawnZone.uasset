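; BP_MonsterSpawnZone spawns a batch of random enemies when a BP_ALTLI_Char overlaps its SpawnTrigger and its SpawnedEnemies list is empty.
; It places AmountToSpawn picks from ClassesToSpawn at random XY points inside the SpawnZone box, at the box's center height.
; Each spawn is tracked in SpawnedEnemies and bound to OnDestroyed, whose handler removes the last spawnActor reference rather than DestroyedActor.
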(event OnComponentBeginOverlap(SpawnTrigger)
  (params (OverlappedComponent :type Primitive%20Component%20Object%20Reference) (OtherActor :type Actor%20Object%20Reference) (OtherComp :type Primitive%20Component%20Object%20Reference) (OtherBodyIndex :type Integer) (bFromSweep :type Boolean) (SweepResult :type Hit%20Result%20Structure%20%28by%20ref%29))
  (bind _spawnzone (Variables|Default|GetSpawnZone))
  (bind _returnvalue (Transformation|GetWorldLocation _spawnzone))
  (bind _boxextent (Variables|/Script/Engine.BoxComponent|GetBoxExtent _spawnzone))
  ;[0.002968 0.09395 1 0.5] Begins spawning enemies when SpawnTrigger is overlapped
  (Utilities|Casting|CastToBP_ALTLI_Char OtherActor ; There might be a more efficient way to\ndo this I'm not sure - Dom
    (:then
      (if (Utilities|Array|IsEmpty (Variables|Default|GetSpawnedEnemies))
        (for _index (range 1 (Variables|Default|GetAmountToSpawn))
          ;[0.002968 0.09395 1 0.5] Spawns an actor (enemy) from the array of class BP_TestEnemy_Base (or other such array)
          (Development|PrintString "spawning")
          (bind _returnvalue_2 (Game|SpawnActorfromClass (.OutItem (Utilities|Array|Random (Variables|Default|GetClassesToSpawn))) (Math|Transform|MakeTransform (Math|Vector|MakeVector (Math|Random|RandomFloatinRange (- (.x _returnvalue) (.x _boxextent)) (+ (.x _returnvalue) (.x _boxextent))) (Math|Random|RandomFloatinRange (- (.y _returnvalue) (.y _boxextent)) (+ (.y _returnvalue) (.y _boxextent))) (.z _returnvalue)) "0, 0, 0" "1.000000,1.000000,1.000000") "AdjustIfPossibleButAlwaysSpawn" "MultiplyWithRoot" 0 0))
          ;[0.002968 0.09395 1 0.5] Removes destroyed enemy from the array of spawned enemies
          (Game|AssignOnDestroyed _returnvalue_2 (delegate Custom|OnDestroyed_Event_0))
          ;[0.002968 0.09395 1 0.5] Adds the spawned enemy to the array of spawned enemies
          (Utilities|Array|Add (Variables|Default|GetSpawnedEnemies) _returnvalue_2)
          (Development|PrintString "added spawned enemy to array"))
        (Development|PrintString "finished spawning")
        (else
          (Development|PrintString "There are still enemies spawned" true true "(R=1.000000,G=0.410883,B=0.000000,A=1.000000)"))))
    (:CastFailed
      (Development|PrintString "ZONE COULD NOT CAST TO CHARACTER" true true "(R=1.000000,G=0.000000,B=0.000000,A=1.000000)"))))

(event Custom|OnDestroyed_Event_0
  (params (DestroyedActor :type Actor%20Object%20Reference))
  ;[0.002968 0.09395 1 0.5] Removes destroyed enemy from the array of spawned enemies
  (Utilities|Array|RemoveItem (Variables|Default|GetSpawnedEnemies) (stale OnComponentBeginOverlap(SpawnTrigger) _returnvalue_2)))

(fn ConstructionScript)