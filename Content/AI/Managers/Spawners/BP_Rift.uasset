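; BP_Rift is an enemy spawner that releases queued enemy classes at its own transform.
; A looping five-second timer spawns the next enemy when the player overlaps the Detection Box.
; Queuing an enemy also triggers an immediate spawn attempt if no test enemy occupies the Spawn Box, regardless of player position.
; Spawned enemies are tracked and bound to a kill event, while the OnEnemyEliminated handler is still empty.
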(event Custom|OnEnemyEliminated)

(event Custom|LookForPlayer
  ;[0.15 0.15 0.15 0.5] Check for the player every five seconds after game start, and spawn enemies if they're within the boundaries of the Detection Box
  (CallFunction|DetectPlayer))

(event EventBeginPlay
  ;[0.15 0.15 0.15 0.5] Check for the player every five seconds after game start, and spawn enemies if they're within the boundaries of the Detection Box
  (Utilities|Time|SetTimerbyEvent (delegate Custom|LookForPlayer) 5.0 true))

(fn ConstructionScript)

(fn SpawnEnemy
  (if (Utilities|Array|IsValidIndex (Variables|Default|GetEnemyQueue))
    (bind _returnvalue (Game|SpawnActorfromClass (Utilities|Array|Get(acopy) (Variables|Default|GetEnemyQueue)) (Transformation|GetActorTransform) "AdjustIfPossibleButAlwaysSpawn" "MultiplyWithRoot" 0 0))
    (Utilities|IsValid _returnvalue
      (:Is%20Valid
        (EventDispatchers|BindEventtoOnKilled _returnvalue (EventDispatchers|CreateEvent :!event Custom|OnEnemyEliminated))
        (Utilities|Array|RemoveIndex (Variables|Default|GetEnemyQueue))
        (Utilities|Array|Add (Variables|Default|GetSpawnedEnemies) _returnvalue)
        (return true)))
    (else
      (Development|PrintString "Enemy not spawned")
      (return false))))

(fn AddEnemytoQueue
  (params (EnemyClass :type BP%20Test%20Enemy%20Base%20Class%20Reference))
  (Utilities|Array|Add (Variables|Default|GetEnemyQueue) EnemyClass)
  (if (not (Utilities|Array|IsValidIndex (Collision|GetOverlappingActors (Variables|Default|GetSpawnBox) "/Game/AI/Enemies/TestingEnemies/BP_TestEnemy_Base.BP_TestEnemy_Base_C" :!class /Script/Engine.PrimitiveComponent)))
    (CallFunction|SpawnEnemy)))

(fn DetectPlayer
  ;[0.15 0.15 0.15 0.5] This should (eventually) detect if the player is inside the Detection Box
  (bind _array_element (Utilities|Array|ForEachLoopwithBreak (Utilities|Array|MakeArray (Variables|Default|GetDetectionBox)) :!label _label)
    (:LoopBody
      (if (Collision|IsOverlappingActor _array_element (Variables|Default|GetPlayer) :!class /Script/Engine.PrimitiveComponent)
        (CallFunction|SpawnEnemy)
        (goto _label Break)
        (else
          (Development|PrintString "Player is not within Detection Box"))))))