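; BP_TestEnemy_Base is a test enemy pawn that wanders the level and dies when the player touches it.
; From BeginPlay it moves via AIMoveTo to random reachable points around itself, re-rolling after a short random delay on success; a failed move only prints a message and ends roaming.
; A capsule overlap with BP_ALTLI_Char destroys the enemy and fires the OnKilled event dispatcher.
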(event OnComponentBeginOverlap(CapsuleComponent)
  (params (OverlappedComponent :type Primitive%20Component%20Object%20Reference) (OtherActor :type Actor%20Object%20Reference) (OtherComp :type Primitive%20Component%20Object%20Reference) (OtherBodyIndex :type Integer) (bFromSweep :type Boolean) (SweepResult :type Hit%20Result%20Structure%20%28by%20ref%29))
  ;[0.15 0.15 0.15 0.5] When the player touches me, I die and call the "OnKilled" event dispatcher
  (Utilities|Casting|CastToBP_ALTLI_Char OtherActor
    (:then
      (Actor|DestroyActor)
      (Default|CallOnKilled))
    (:CastFailed
      (Development|PrintString "Could not cast to Character"))))

(event Custom|RandomRoam
  ;[0.15 0.15 0.15 0.5] Lets the test AI roam around the play area
  (AI|AIMoveTo self (.RandomLocation (AI|Navigation|GetRandomReachablePointinRadius (Transformation|GetActorLocation) 2e+03 0 0)) 0 5.0 false
    (:OnSuccess
      (Utilities|FlowControl|Delay (Math|Random|RandomFloatinRange 0.2 1.0))
      (CallFunction|RandomRoam))
    (:OnFail
      (Development|PrintString "COULD NOT MOVE!!!"))))

(event EventBeginPlay
  ;[0.15 0.15 0.15 0.5] On BeginPlay, begin roaming
  (CallFunction|RandomRoam))

(fn ConstructionScript)