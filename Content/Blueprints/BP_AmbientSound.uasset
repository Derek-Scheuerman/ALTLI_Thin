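; BP_AmbientSound is an actor that plays a configurable ambient sound or music track in the level.
; On BeginPlay it spawns the Sound at its root's location, stores the audio component and immediately sets its volume to VolumeLevel.
; The ChangeMusic event is empty, and an unconnected switch that would swap the playing sound to the starter music cue or none never runs.
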(event Custom|Change%20Music
  (params (MusicSelect :type Integer)))

(event EventBeginPlay
  (bind _returnvalue (Audio|SpawnSoundatLocation (Variables|Default|GetSound) (Transformation|GetWorldLocation (Variables|Default|GetDefaultSceneRoot)) "0, 0, 0" 1.0 1.0 0.0 0 0))
  (bind _output_get (Variables|Default|SetSoundBeingPlayed _returnvalue))
  (Audio|Components|Audio|AdjustVolume _output_get 0.0 (Variables|Default|GetVolumeLevel) "Linear" :!class /Script/Engine.AudioComponent))

(event Collision|EventActorBeginOverlap
  (params (OtherActor :type Actor%20Object%20Reference)))

(event EventTick
  (params (DeltaSeconds :type Float%20%28single-precision%29)))

(fn ConstructionScript)