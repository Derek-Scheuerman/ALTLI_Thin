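; BP_GateLever is an interactable lever that opens its referenced Gate and visibly flips between two positions.
; InteractWith calls OpenSesame on the Gate on every use, then runs Flip, while LookAt returns an empty string.
; Flip picks one of two timelines by the Pulled flag, lerping the pivot's roll from its current value toward either tilt, and updates Pulled only when finished.
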(event Custom|Flip
  (bind _bp_leverpivottest (Variables|Default|GetBP_LeverPivotTest))
  (bind _bp_leverpivottest_2 (Variables|Default|GetBP_LeverPivotTest))
  (if (Variables|Default|GetPulled)
    (bind _newtrack_0 (Timeline|Timeline_1 PlayFromStart)
      (:Update
        (Transformation|SetRelativeRotation _bp_leverpivottest (Math|Rotator|MakeRotator (Math|Float|Lerp (.roll (Variables|/Script/Engine.SceneComponent|GetRelativeRotation _bp_leverpivottest)) 4e+01 _newtrack_0) 0.0 0.0) false false))
      (:Finished
        (Variables|Default|SetPulled false)
        (Development|PrintString "Done")))
    (else
      (bind _newtrack_0_2 (Timeline|Timeline_0 PlayFromStart)
        (:Update
          (Transformation|SetRelativeRotation _bp_leverpivottest_2 (Math|Rotator|MakeRotator (Math|Float|Lerp (.roll (Variables|/Script/Engine.SceneComponent|GetRelativeRotation _bp_leverpivottest_2)) -4e+01 _newtrack_0_2) 0.0 0.0) false false))
        (:Finished
          (Variables|Default|SetPulled true)
          (Development|PrintString "Done"))))))

(event EventBeginPlay)

(event Collision|EventActorBeginOverlap
  (params (OtherActor :type Actor%20Object%20Reference)))

(event EventTick
  (params (DeltaSeconds :type Float%20%28single-precision%29)))

(fn ConstructionScript)

(fn Interactwith
  (params (PlayerC :type BP%20ALTLI%20Char%20Object%20Reference))
  (Default|OpenSesame (Variables|Default|GetGate))
  (CallFunction|Flip)
  (return "" 0))

(fn Lookat
  (return ""))