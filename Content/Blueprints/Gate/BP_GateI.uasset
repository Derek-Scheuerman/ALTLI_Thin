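; Gate actor that swings its Gate component between raised and lowered positions each time the OpenSesame event is called.
; The Down flag selects one of two timelines, which lerp the roll from its current value toward 0 or -90 degrees.
; Each timeline flips Down when it finishes, with debug prints reporting the state.
; BeginPlay, the construction script and SpinTheWheel are empty.
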(event Custom|Open%20Sesame
  (bind _gate (Variables|Default|GetGate))
  (bind _gate_2 (Variables|Default|GetGate))
  (if (Variables|Default|GetbDown)
    (bind _newtrack_0 (Timeline|Timeline PlayFromStart)
      (:Update
        (Transformation|SetRelativeRotation _gate (Math|Rotator|MakeRotator (Math|Float|Lerp (.roll (Variables|/Script/Engine.SceneComponent|GetRelativeRotation _gate)) 0.0 _newtrack_0) 0.0 0.0) false false))
      (:Finished
        (if (Variables|Default|GetbDown)
          (Variables|Default|SetbDown false)
          (Development|PrintString "Up")
          (else
            (Variables|Default|SetbDown true)))))
    (else
      (bind _newtrack_0_2 (Timeline|Open PlayFromStart)
        (:Update
          (Transformation|SetRelativeRotation _gate_2 (Math|Rotator|MakeRotator (Math|Float|Lerp (.roll (Variables|/Script/Engine.SceneComponent|GetRelativeRotation _gate_2)) -9e+01 _newtrack_0_2) 0.0 0.0) false false))
        (:Finished
          (if (Variables|Default|GetbDown)
            (Variables|Default|SetbDown false)
            (Development|PrintString "Up!")
            (else
              (Variables|Default|SetbDown true)
              (Development|PrintString "Down!"))))))))

(event EventBeginPlay)

(event Collision|EventActorBeginOverlap
  (params (OtherActor :type Actor%20Object%20Reference)))

(event EventTick
  (params (DeltaSeconds :type Float%20%28single-precision%29)))

(fn ConstructionScript)

(fn SpintheWheel)