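; Rat actor that runs its skeletal mesh along a spline path on repeat, with a random pause between runs.
; BeginPlay sets the spline duration and starts FollowPath, which re-calls itself through a frame-length Delay instead of using Tick.
; Each step samples the spline at constant velocity, aligning the mesh to its direction with a yaw offset.
; At the end, time resets and the next run restarts after the wait.
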(event Custom|FollowPath
  (bind _spline (Variables|Default|GetSpline))
  (bind _output_get (Variables|Default|SetCurrTime (+ (Utilities|Time|GetWorldDeltaSeconds) (Variables|Default|GetCurrTime))))
  (Transformation|SetWorldLocationAndRotation (Variables|Default|GetSkeletalMesh) (Spline|GetLocationatTime _spline _output_get "World" true) (Math|Rotator|MakeRotator (.Roll (Math|Rotator|BreakRotator (Math|Rotator|MakeRotfromX (Class|SplineComponent|GetDirectionatTime _spline _output_get "World" true)))) (.Pitch (Math|Rotator|BreakRotator (Math|Rotator|MakeRotfromX (Class|SplineComponent|GetDirectionatTime _spline _output_get "World" true)))) (+ (.Yaw (Math|Rotator|BreakRotator (Math|Rotator|MakeRotfromX (Class|SplineComponent|GetDirectionatTime _spline _output_get "World" true)))) -9e+01)) false false)
  (if (>= (Variables|Default|GetCurrTime) (Variables|RatControls|GetSplineDuration))
    (Variables|Default|SetCurrTime 0.0)
    (Utilities|FlowControl|Delay (Math|Random|RandomFloatinRange (Variables|RatControls|GetMinWaitTime) (Variables|RatControls|GetMaxWaitTime)))
    (CallFunction|FollowPath)
    (else
      (Utilities|FlowControl|Delay (Utilities|Time|GetWorldDeltaSeconds))
      (CallFunction|FollowPath))))

(event EventBeginPlay
  (Variables|/Script/Engine.SplineComponent|SetDuration (Variables|Default|GetSpline) (Variables|RatControls|GetSplineDuration))
  (CallFunction|FollowPath))

(fn ConstructionScript)