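; Actor component that turns its owner into a pickup item for the inventory system, holding item ID, quantity and durability.
; On BeginPlay it enables replication on the owner and seeds durability from the item's data table row.
; InteractWith adds the item to the player's inventory component and destroys the owner on success.
; Durability has get, set and additive update functions, while LookAt and the objective outputs return empty values.
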(event EventBeginPlay
  (Networking|SetReplicates (Components|GetOwner) true)
  (bind _returnvalue (Utilities|GetDataTableRow "/Game/Blueprints/Inventory/Item_Data.Item_Data" (.rowname (Variables|Default|GetItemID)))
    (:then
      (CallFunction|SetDurability (.Durability (Utilities|Struct|BreakFItemStruct _returnvalue))))))

(fn GetDurability
  (return (Variables|Default|GetDurability)))

(fn SetDurability
  (params (Durability :type Float%20%28double-precision%29))
  (Variables|Default|SetDurability Durability))

(fn UpdateDurability
  (params (Change :type Float%20%28double-precision%29))
  (bind _output_get (Variables|Default|SetDurability (+ Change (Variables|Default|GetDurability))))
  (return _output_get))

(fn Interactwith
  (params (PlayerC :type BP%20ALTLI%20Char%20Object%20Reference))
  (bind _ac_inventorysystem (Variables|/Game/Characters/FirstPerson/Blueprints/BP_ALTLI_Char.BP_ALTLI_Char_C|GetAC_InventorySystem PlayerC))
  (Utilities|IsValid _ac_inventorysystem
    (:Is%20Valid
      (bind _seccess (Default|AddtoInv _ac_inventorysystem (.rowname (Variables|Default|GetItemID)) (Variables|Default|GetQuantity)))
      (if _seccess
        (Actor|DestroyActor (Components|GetOwner))
        (return "" 0)))))

(fn Lookat
  (return ""))