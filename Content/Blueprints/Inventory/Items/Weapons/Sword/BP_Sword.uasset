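; Sword weapon item that players equip, sheathe, drop and swing, and that enemies can also swing.
; Item data loads a data table row that sets damage, tier modifier and cooldown.
; Player and enemy swings share one montage path with different trace channels, where notifies toggle the DidItHitActor trace.
; Hits apply randomized point damage scaled by instigator, sword and tier, and report a damage event.
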(event Custom|HitActorOnSwordSwing
  (params (LastItem :type Hit%20Result%20Structure))
  (bind (_bblockinghit _binitialoverlap _time _distance _location _impactpoint _normal _impactnormal _physmat _hitactor _hitcomponent _hitbonename _bonename _hititem _elementindex _faceindex _tracestart) (Collision|BreakHitResult LastItem))
  (bind _sword_data_damage (CallFunction|GetDamageModifier))
  (bind _swordtiermodifier (Variables|Default|GetSwordTierModifier))
  (bind _instigator_damage (Variables|Default|GetInstigator%20Damage))
  (bind _returnvalue (* _sword_data_damage _instigator_damage))
  (bind _returnvalue_2 (* _returnvalue _swordtiermodifier))
  (bind _returnvalue_3 (* _returnvalue_2 0.75))
  (bind _returnvalue_4 (Math|Random|RandomFloatinRange _returnvalue_3 _returnvalue_2))
  ;[0.15 0.09801 0 0.5] Process Hit actor and damage
  (Game|Damage|ApplyPointDamage _hitactor _returnvalue_4 _tracestart LastItem (Game|GetInstigatorController (Variables|Default|GetSwingInstigator)))
  (Class|AISenseDamage|ReportDamageEvent _hitactor (Variables|Default|GetSwingInstigator) _returnvalue_4 _tracestart "0, 0, 0" "Sword"))

(event Custom|EnemySwing
  (params (SwingInstigator :type Character%20Object%20Reference) (InstigatorDamage :type Float%20%28double-precision%29))
  (bind _swingmontage (Variables|Default|GetSwingMontage))
  (bind _swordcooldown (Variables|Default|GetSwordCoolDown))
  (bind _player_ref (Variables|Default|GetPlayer%20Ref))
  (bind _returnvalue (Animation|GetPlayLength _swingmontage))
  (bind _returnvalue_2 (- _swordcooldown _returnvalue))
  ;[0 1 0.7277 0.5] Swing Sword
  ;;[0.5767 0 0.02784 0.5] Enemy swing
  (Variables|Default|SetSwingInstigator SwingInstigator)
  (Variables|Default|SetInstigator%20Damage InstigatorDamage)
  (Variables|/Script/DidItHit.DidItHitActorComponent|SetMyTraceChannel (Variables|Default|GetDidItHitActor) "TraceTypeQuery4")
  (if (< _returnvalue_2 0.0)
    ;;[0 0.6176 0.95 0.5] Swing speed
    (Variables|Default|SetSwingAnimPlayRate (+ (- (Animation|GetPlayLength (Variables|Default|GetSwingMontage)) (Variables|Default|GetSwordCoolDown)) 1.0)))
  (bind _notifyname (Animation|Montage|PlayMontage (Variables|/Script/Engine.Character|GetMesh (Variables|Default|GetSwingInstigator)) (Variables|Default|GetSwingMontage) (Variables|Default|GetSwingAnimPlayRate))
    (:then
      ;;[0.15 0.1033 0.04113 0.5] Player is swinging
      (if (== (Variables|Default|GetSwingInstigator) (Variables|Default|GetPlayer%20Ref))
        (Variables|/Game/Characters/FirstPerson/Blueprints/BP_ALTLI_Char.BP_ALTLI_Char_C|SetIsAttacking _player_ref true)))
    (:OnCompleted
      (Utilities|FlowControl|Delay _returnvalue_2 :!label _label)
      (if (== (Variables|Default|GetSwingInstigator) _player_ref)
        (Variables|/Game/Characters/FirstPerson/Blueprints/BP_ALTLI_Char.BP_ALTLI_Char_C|SetIsAttacking _player_ref false)
        (else
          (Utilities|Casting|CastToBP_EnemyMain (Variables|Default|GetSwingInstigator))))
      (Class|DidItHitActorComponent|ToggleTraceCheck (Variables|Default|GetDidItHitActor) false :!label _label_2)
      (Class|DidItHitActorComponent|ClearHitArray (Variables|Default|GetDidItHitActor)))
    (:OnInterrupted
      (goto _label))
    (:OnNotifyBegin
      (if (== _notifyname "SwingStart")
        (Class|DidItHitActorComponent|ToggleTraceCheck (Variables|Default|GetDidItHitActor) true)
        ;;[0.02202 0.15 0.04304 0.5] Play sound
        (Audio|PlaySoundatLocation "/Engine/VREditor/Sounds/VR_ungrab_Cue.VR_ungrab_Cue" (Transformation|GetActorLocation) "0, 0, 0" 1.0 1.0 0.0 0 0 0 0)
        (elif (== _notifyname "SwingEnd")
          (goto _label_2))))))

(event EventBeginPlay
  (bind _didithitactor (Variables|Default|GetDidItHitActor))
  (Class|DidItHitActorComponent|SetupVariables _didithitactor (Variables|Default|GetStaticMesh))
  (EventDispatchers|BindEventtoOnItemAdded _didithitactor (EventDispatchers|CreateEvent :!event Custom|HitActorOnSwordSwing)))

(event EventEquip
  (params (PlayerRef :type BP%20ALTLI%20Char%20Object%20Reference) (ItemIndex :type Integer))
  ;[0.7448 0 0.478 0.5] Equip Sword
  (bind _output_get (Variables|Default|SetPlayer%20Ref PlayerRef))
  (Variables|/Game/Characters/FirstPerson/Blueprints/BP_ALTLI_Char.BP_ALTLI_Char_C|SetHeldItemRight _output_get self)
  (Variables|/Game/Characters/FirstPerson/Blueprints/BP_ALTLI_Char.BP_ALTLI_Char_C|SetHeldItemRightIndex (Variables|Default|GetPlayer%20Ref) ItemIndex)
  (Rendering|SetVisibility (Variables|Default|GetStaticMesh) false true)
  (Variables|/Game/Characters/FirstPerson/Blueprints/BP_ALTLI_Char.BP_ALTLI_Char_C|SetisHoldingItemRight (Variables|Default|GetPlayer%20Ref) true)
  (Variables|Default|SetPlayerLevel (.Value (Utilities|Map|Find (Variables|/Game/Characters/FirstPerson/Blueprints/BP_ALTLI_Char.BP_ALTLI_Char_C|GetLevels (Variables|Default|GetPlayer%20Ref)) "NewEnumerator4")))
  (Utilities|FlowControl|FlipFlop
    (:A
      (Physics|SetSimulatePhysics (Variables|Default|GetStaticMesh) false)
      (Transformation|AttachComponentToComponent (Variables|/Script/Engine.Character|GetMesh (Variables|Default|GetPlayer%20Ref)) "HandGrip_R" "SnapToTarget" "SnapToTarget" "SnapToTarget" true)
      (Rendering|SetVisibility (Variables|Default|GetStaticMesh) true true)
      (Animation|Montage|PlayMontage (Variables|/Script/Engine.Character|GetMesh (Variables|Default|GetPlayer%20Ref)) "/Game/Blueprints/Inventory/Items/Weapons/Sword/Anim/Unsheath_Sword_Anim_Montage.Unsheath_Sword_Anim_Montage" 1.0 0.0 "None" false))
    (:B
      (Rendering|SetVisibility (Variables|Default|GetStaticMesh) true true)
      (Animation|Montage|PlayMontage (Variables|/Script/Engine.Character|GetMesh (Variables|Default|GetPlayer%20Ref)) "/Game/Blueprints/Inventory/Items/Weapons/Sword/Anim/Sheath_Sword_Anim_Montage.Sheath_Sword_Anim_Montage" 1.0 0.0 "None" false
        (:OnCompleted
          (Variables|/Game/Characters/FirstPerson/Blueprints/BP_ALTLI_Char.BP_ALTLI_Char_C|SetisHoldingItemRight (Variables|Default|GetPlayer%20Ref) false)
          (Variables|/Game/Characters/FirstPerson/Blueprints/BP_ALTLI_Char.BP_ALTLI_Char_C|SetHeldItemRight (Variables|Default|GetPlayer%20Ref) 0)
          (Actor|DestroyActor))))))

(event EventDrop
  (bind _staticmesh (Variables|Default|GetStaticMesh))
  ;[0.03832 0.15 0 0.5] Dropping sword
  (Transformation|DetachFromActor "KeepWorld" "KeepWorld" "KeepRelative")
  (Collision|SetCollisionEnabled _staticmesh "QueryAndPhysics")
  (Physics|SetSimulatePhysics _staticmesh true))

(event EventSetItemData
  (params (ItemData :type F%20Slot%20Struct%20Structure))
  ;[0.15 0.15 0.15 0.5] Setup sword data
  (Variables|/Game/Blueprints/Inventory/ItemDataComponent.ItemDataComponent_C|SetItemID (Variables|Default|GetItemDataComponent) (Utilities|Struct|MakeDataTableRowHandle "/Game/Blueprints/Inventory/ALTLI_Leveling_-_Item_Data_sheet.ALTLI_Leveling_-_Item_Data_sheet" (.itemid ItemData)))
  (Variables|Default|SetDurability (.durability ItemData))
  (bind _returnvalue (Utilities|GetDataTableRow (.datatable (Variables|/Game/Blueprints/Inventory/ItemDataComponent.ItemDataComponent_C|GetItemID (Variables|Default|GetItemDataComponent))) (.rowname (Variables|/Game/Blueprints/Inventory/ItemDataComponent.ItemDataComponent_C|GetItemID (Variables|Default|GetItemDataComponent))))
    (:then
      (Variables|Default|SetSwordData _returnvalue)
      (CallFunction|SetCoolDown 0.0)
      (CallFunction|SetTypeModifier))))

(event EventUsePrimary
  (params (instigator :type BP%20ALTLI%20Char%20Object%20Reference) (InputType :type E_PlayerInputType%20Enum :default "NewEnumerator0") (TriggeredSecs :type Float%20%28double-precision%29))
  (bind _player_ref (Variables|Default|GetPlayer%20Ref))
  (bind _swingmontage (Variables|Default|GetSwingMontage))
  (bind _swordcooldown (Variables|Default|GetSwordCoolDown))
  (bind _player_ref_2 (Variables|Default|GetPlayer%20Ref))
  (bind _returnvalue (Animation|GetPlayLength _swingmontage))
  (bind _returnvalue_2 (- _swordcooldown _returnvalue))
  ;[0 1 0.7277 0.5] Swing Sword
  ;;[0.15 0.1215 0.03276 0.5] PlayerSwing
  (Variables|Default|SetSwingInstigator instigator)
  (Variables|Default|SetInstigator%20Damage (Variables|/Game/Characters/FirstPerson/Blueprints/BP_ALTLI_Char.BP_ALTLI_Char_C|GetDamage _player_ref))
  (if (not (Variables|/Game/Characters/FirstPerson/Blueprints/BP_ALTLI_Char.BP_ALTLI_Char_C|GetIsAttacking _player_ref))
    (Variables|/Game/Characters/FirstPerson/Blueprints/BP_ALTLI_Char.BP_ALTLI_Char_C|SetIsAttacking _player_ref true)
    (Variables|/Script/DidItHit.DidItHitActorComponent|SetMyTraceChannel (Variables|Default|GetDidItHitActor) "TraceTypeQuery3")
    (if (< _returnvalue_2 0.0)
      ;;[0 0.6176 0.95 0.5] Swing speed
      (Variables|Default|SetSwingAnimPlayRate (+ (- (Animation|GetPlayLength (Variables|Default|GetSwingMontage)) (Variables|Default|GetSwordCoolDown)) 1.0)))
    (bind _notifyname (Animation|Montage|PlayMontage (Variables|/Script/Engine.Character|GetMesh (Variables|Default|GetSwingInstigator)) (Variables|Default|GetSwingMontage) (Variables|Default|GetSwingAnimPlayRate))
      (:then
        ;;[0.15 0.1033 0.04113 0.5] Player is swinging
        (if (== (Variables|Default|GetSwingInstigator) (Variables|Default|GetPlayer%20Ref))
          (Variables|/Game/Characters/FirstPerson/Blueprints/BP_ALTLI_Char.BP_ALTLI_Char_C|SetIsAttacking _player_ref_2 true)))
      (:OnCompleted
        (Utilities|FlowControl|Delay _returnvalue_2 :!label _label)
        (if (== (Variables|Default|GetSwingInstigator) _player_ref_2)
          (Variables|/Game/Characters/FirstPerson/Blueprints/BP_ALTLI_Char.BP_ALTLI_Char_C|SetIsAttacking _player_ref_2 false)
          (else
            (Utilities|Casting|CastToBP_EnemyMain (Variables|Default|GetSwingInstigator))))
        (Class|DidItHitActorComponent|ToggleTraceCheck (Variables|Default|GetDidItHitActor) false :!label _label_2)
        (Class|DidItHitActorComponent|ClearHitArray (Variables|Default|GetDidItHitActor)))
      (:OnInterrupted
        (goto _label))
      (:OnNotifyBegin
        (if (== _notifyname "SwingStart")
          (Class|DidItHitActorComponent|ToggleTraceCheck (Variables|Default|GetDidItHitActor) true)
          ;;[0.02202 0.15 0.04304 0.5] Play sound
          (Audio|PlaySoundatLocation "/Engine/VREditor/Sounds/VR_ungrab_Cue.VR_ungrab_Cue" (Transformation|GetActorLocation) "0, 0, 0" 1.0 1.0 0.0 0 0 0 0)
          (elif (== _notifyname "SwingEnd")
            (goto _label_2)))))))

(fn ConstructionScript
  (|CallParentFunction))

(fn GetDamageModifier
  (return (.damage (Variables|Default|GetSwordData))))

(fn SetTypeModifier
  (bind _output_get (Variables|Default|SetSwordTierModifier (+ (/ (Math|Conversions|ToFloat(Integer) (Math|Conversions|ToInteger(Byte) (.tiermodifier (Variables|Default|GetSwordData)))) 1e+01) 1.0)))
  (return _output_get))

(fn SetCoolDown
  (params (CoolDown :type Float%20%28double-precision%29))
  (if (!= CoolDown 0.0)
    (Variables|Default|SetSwordCoolDown CoolDown)
    (else
      (Variables|Default|SetSwordCoolDown (.secondsperhit (Variables|Default|GetSwordData))))))