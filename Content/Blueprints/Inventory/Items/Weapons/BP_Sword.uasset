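; Sword weapon item that the player equips in the right hand from the hotbar, slashes with and can drop as a physics object.
; Equip registers it on the player, then a FlipFlop alternates between attaching it with an unsheath montage and sheathing it before destroying the actor.
; Primary use plays a slash montage whose notify runs a forward sphere trace, applying player-scaled damage to interface-implementing actors and reporting it to AI, with a cooldown after completion.
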(event EventBeginPlay)

(event EventEquip
  (params (PlayerRef :type BP%20ALTLI%20Char%20Object%20Reference) (HotBarIndex :type Integer))
  ;[0.7448 0 0.478 0.5] Equip Sword
  (bind _output_get (Variables|Default|SetPlayer%20Ref PlayerRef))
  (Variables|/Game/Characters/FirstPerson/Blueprints/BP_ALTLI_Char.BP_ALTLI_Char_C|SetHeldItemRight _output_get self)
  (Variables|/Game/Characters/FirstPerson/Blueprints/BP_ALTLI_Char.BP_ALTLI_Char_C|SetHeldItemRightIndex (Variables|Default|GetPlayer%20Ref) HotBarIndex)
  (Rendering|SetVisibility (Variables|Default|GetStaticMesh) false true)
  (Variables|/Game/Characters/FirstPerson/Blueprints/BP_ALTLI_Char.BP_ALTLI_Char_C|SetisHoldingItemRight (Variables|Default|GetPlayer%20Ref) true)
  (Variables|Default|SetPlayerLevel (Variables|/Game/Characters/FirstPerson/Blueprints/BP_ALTLI_Char.BP_ALTLI_Char_C|GetLevel (Variables|Default|GetPlayer%20Ref)))
  (Utilities|FlowControl|FlipFlop
    (:A
      (Physics|SetSimulatePhysics (Variables|Default|GetStaticMesh) false)
      (Transformation|AttachComponentToComponent (Variables|/Script/Engine.Character|GetMesh (Variables|Default|GetPlayer%20Ref)) "HandGrip_R" "SnapToTarget" "SnapToTarget" "SnapToTarget" true)
      (Rendering|SetVisibility (Variables|Default|GetStaticMesh) true true)
      (Animation|Montage|PlayMontage (Variables|/Script/Engine.Character|GetMesh (Variables|Default|GetPlayer%20Ref)) "/Game/Blueprints/Inventory/Items/Weapons/Unsheath_Sword_Anim_Montage.Unsheath_Sword_Anim_Montage" 1.0 0.0 "None" false))
    (:B
      (Rendering|SetVisibility (Variables|Default|GetStaticMesh) true true)
      (Animation|Montage|PlayMontage (Variables|/Script/Engine.Character|GetMesh (Variables|Default|GetPlayer%20Ref)) "/Game/Blueprints/Inventory/Items/Weapons/Sheath_Sword_Anim_Montage.Sheath_Sword_Anim_Montage" 1.0 0.0 "None" false
        (:OnCompleted
          (Variables|/Game/Characters/FirstPerson/Blueprints/BP_ALTLI_Char.BP_ALTLI_Char_C|SetisHoldingItemRight (Variables|Default|GetPlayer%20Ref) false)
          (Variables|/Game/Characters/FirstPerson/Blueprints/BP_ALTLI_Char.BP_ALTLI_Char_C|SetHeldItemRight (Variables|Default|GetPlayer%20Ref) 0)
          (Actor|DestroyActor))))))

(event EventDrop
  (bind _staticmesh (Variables|Default|GetStaticMesh))
  (Transformation|DetachFromActor "KeepWorld" "KeepWorld" "KeepRelative")
  (Collision|SetCollisionEnabled _staticmesh "QueryAndPhysics")
  (Physics|SetSimulatePhysics _staticmesh true))

(event EventUsePrimary
  (params (instigator :type BP%20ALTLI%20Char%20Object%20Reference) (InputType :type E_PlayerInputType%20Enum :default "NewEnumerator0"))
  (bind _returnvalue (Transformation|GetActorLocation))
  (bind _player_ref (Variables|Default|GetPlayer%20Ref))
  (bind _damage_sword (Variables|Default|GetDamage_Sword))
  (bind _player_ref_2 (Variables|Default|GetPlayer%20Ref))
  (bind _base_damage (Variables|/Game/Characters/FirstPerson/Blueprints/BP_ALTLI_Char.BP_ALTLI_Char_C|GetBase_Damage _player_ref))
  (bind _returnvalue_2 (* _damage_sword _base_damage))
  (if (not (Variables|/Game/Characters/FirstPerson/Blueprints/BP_ALTLI_Char.BP_ALTLI_Char_C|GetIsAttacking _player_ref_2))
    (Variables|/Game/Characters/FirstPerson/Blueprints/BP_ALTLI_Char.BP_ALTLI_Char_C|SetIsAttacking _player_ref_2 true)
    (Animation|Montage|PlayMontage (Variables|/Script/Engine.Character|GetMesh (Variables|Default|GetPlayer%20Ref)) "/Game/Blueprints/Inventory/Items/Weapons/Sword_And_Shield_Slash_Anim_Montage.Sword_And_Shield_Slash_Anim_Montage"
      (:OnCompleted
        (Utilities|FlowControl|Delay (Variables|Default|GetSwordCoolDown))
        (Variables|/Game/Characters/FirstPerson/Blueprints/BP_ALTLI_Char.BP_ALTLI_Char_C|SetIsAttacking (Variables|Default|GetPlayer%20Ref) false))
      (:OnNotifyBegin
        (Audio|PlaySoundatLocation 0 (Transformation|GetActorLocation) "0, 0, 0" 1.0 1.0 0.0 0 0 0 0)
        (Audio|PlaySoundatLocation 0 _returnvalue "0, 0, 0" 1.0 1.0 0.0 0 0 0 0)
        (bind (_outhits _returnvalue_3) (Collision|MultiSphereTraceByChannel _returnvalue (+ _returnvalue (* (Transformation|GetActorForwardVector) (Variables|Default|GetSwordReach))) 1.2e+02 "TraceTypeQuery4" false 0 "None"))
        (if _returnvalue_3
          (for _array_element _outhits
            (if (Utilities|DoesObjectImplementInterface (.HitActor (Collision|BreakHitResult _array_element)) 0)
              (Game|Damage|ApplyPointDamage (.HitActor (Collision|BreakHitResult _array_element)) _returnvalue_2 (.TraceStart (Collision|BreakHitResult _array_element)) _array_element (Game|GetInstigatorController instigator))
              (Class|AISenseDamage|ReportDamageEvent (.HitActor (Collision|BreakHitResult _array_element)) instigator _returnvalue_2 (.TraceStart (Collision|BreakHitResult _array_element)) "0, 0, 0" "Sword"))))))))

(fn ConstructionScript
  (|CallParentFunction))