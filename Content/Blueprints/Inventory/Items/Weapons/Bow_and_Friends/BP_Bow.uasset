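; Bow weapon item that attaches to the player's right hand on equip and sheathes and destroys itself on the next toggle.
; Drawing checks cooldown and arrow count; firing spawns an arrow aimed by a camera line trace, with level-scaled damage, and spends ammo and durability.
; Destruction records the actor in the game mode's save data.
; Draw and fire montages are unwired, and Break sets Broken to false.
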(event Custom|Draw%20Bow
  ;[0.15 0.15 0.15 0.5] If the Cooldown is Expired and we have arrows, play the animation and draw!
  (if (> (- (Utilities|Time|GetGameTimeinSeconds) (Variables|Default|GetTime%20of%20Last%20Shot)) (Variables|CanYouFire?|GetCooldown))
    (if (> (Variables|CanYouFire?|GetCurrent%20Arrows) 0)
      (Variables|CanYouFire?|SetbIsDrawn true)
      (Development|PrintString "REALLY drawn!"))))

(event Custom|Fire%20Bow
  ;[0.15 0.15 0.15 0.5] If the Bow is drawn, feel free to fire
  (if (Variables|CanYouFire?|GetbIsDrawn)
    (CallFunction|FireArrow)
    (Variables|CanYouFire?|SetTime%20Of%20Last%20Shot (Utilities|Time|GetGameTimeinSeconds))))

(event Custom|Fire%20Arrow
  ;[1 0 0.006618 0.5] Literally Spawn in the Arrow and Decrement the Arrow Count
  (CallFunction|PlayFireMontage)
  (bind _newparam (CallFunction|GetWeaponTarget))
  (bind _newparam_2 (CallFunction|CalculateArrowSpawnTransform _newparam))
  (bind _returnvalue (Game|SpawnActorfromClass (Variables|Default|GetArrow) _newparam_2 "Undefined" "MultiplyWithRoot" (Variables|Default|GetPlayer%20Ref) (Variables|Default|GetPlayer%20Ref)))
  (Components|Activation|Activate (Variables|/Game/Blueprints/Inventory/Items/Weapons/Bow_and_Friends/BP_ArrowNew.BP_ArrowNew_C|GetProjectileMovement _returnvalue) false)
  (Variables|/Game/Blueprints/Inventory/Items/Weapons/Bow_and_Friends/BP_ArrowNew.BP_ArrowNew_C|SetDamage _returnvalue (* (Variables|Damage|GetBase%20Damage) (Variables|Damage|GetDamage%20Modifier) (Variables|Damage|GetLevel)))
  (Math|Integer|DecrementInt (Variables|CanYouFire?|GetCurrent%20Arrows)
    (:%20%20
      (Math|Float|DecrementFloat (Variables|NonCombatStats|GetDurability)
        (:%20%20
          (Variables|CanYouFire?|SetbIsDrawn false))))))

(event Custom|Reload
  ;[0.15 0.15 0.15 0.5] Increment Arrows when Reloading
  (if (< (Variables|CanYouFire?|GetCurrent%20Arrows) 1)
    (Utilities|FlowControl|Delay 1.0)
    (Math|Integer|IncrementInt (Variables|CanYouFire?|GetCurrent%20Arrows))))

(event Custom|Undraw%20Bow
  (Variables|CanYouFire?|SetbIsDrawn false))

(event Custom|Play%20Fire%20Montage)

(event Custom|Activate%20Weapon
  ;[0.15 0.15 0.15 0.5] Literally make the weapon visible when activated
  (Rendering|SetActorHiddenInGame false))

(event Custom|Break
  (Variables|CanYouFire?|SetBroken false))

(event EventDrop
  (bind _bowmesh (Variables|Default|GetBowMesh))
  (Transformation|DetachFromActor "KeepWorld" "KeepWorld" "KeepRelative")
  (Collision|SetCollisionEnabled _bowmesh "QueryAndPhysics")
  (Physics|SetSimulatePhysics _bowmesh true))

(event EventBeginPlay)

(event EventDestroyed
  (bind _asbp_altli_mode (Utilities|Casting|CastToBP_ALTLI_Mode (Game|GetGameMode)))
  (Utilities|Array|AddUnique (Variables|/Game/SG_ALTLI_Data.SG_ALTLI_Data_C|GetActorsRemoved (Variables|/Game/Characters/FirstPerson/Blueprints/BP_ALTLI_Mode.BP_ALTLI_Mode_C|GetSaveData _asbp_altli_mode)) (Utilities|ResolveSoftReference self)))

(event EventUsePrimary
  (params (instigator :type BP%20ALTLI%20Char%20Object%20Reference) (InputType :type E_PlayerInputType%20Enum :default "NewEnumerator0"))
  ;[1 0.8505 0 0.5] Inputs to Use the Thing
  (if (Utilities|Enum|Equal(Enum) InputType "NewEnumerator1")
    (if (Utilities|Enum|Equal(Enum) (stale EventUseSecondary InputType) "NewEnumerator4")
      (CallFunction|FireBow))))

(event EventUseSecondary
  (params (InputType :type E_PlayerInputType%20Enum :default "NewEnumerator0") (Instigator :type BP%20ALTLI%20Char%20Object%20Reference))
  ;[1 0.8505 0 0.5] Inputs to Use the Thing
  (if (Utilities|Enum|Equal(Enum) InputType "NewEnumerator1")
    (if (or (Utilities|Enum|Equal(Enum) InputType "NewEnumerator4") (Utilities|Enum|Equal(Enum) InputType "NewEnumerator3"))
      (CallFunction|UndrawBow)
      (Development|PrintString "undraw")
      (elif (Variables|CanYouFire?|GetBroken)
        (Development|PrintString "It's Broken!")
        (else
          (CallFunction|DrawBow)
          (Development|PrintString "Drawn"))))))

(event EventEquip
  (params (PlayerRef :type BP%20ALTLI%20Char%20Object%20Reference) (HotBarIndex :type Integer))
  (bind _output_get (Variables|Default|SetPlayer%20Ref PlayerRef))
  (Variables|/Game/Characters/FirstPerson/Blueprints/BP_ALTLI_Char.BP_ALTLI_Char_C|SetHeldItemRight _output_get self)
  (Variables|/Game/Characters/FirstPerson/Blueprints/BP_ALTLI_Char.BP_ALTLI_Char_C|SetHeldItemRightIndex (Variables|Default|GetPlayer%20Ref) HotBarIndex)
  (Rendering|SetVisibility (Variables|Default|GetBowMesh) false true)
  (Variables|/Game/Characters/FirstPerson/Blueprints/BP_ALTLI_Char.BP_ALTLI_Char_C|SetisHoldingItemRight (Variables|Default|GetPlayer%20Ref) true)
  (Variables|Damage|SetLevel (Variables|/Game/Characters/FirstPerson/Blueprints/BP_ALTLI_Char.BP_ALTLI_Char_C|GetLevel (Variables|Default|GetPlayer%20Ref)))
  (Utilities|FlowControl|FlipFlop
    (:A
      (Physics|SetSimulatePhysics (Variables|Default|GetBowMesh) false)
      (Transformation|AttachComponentToComponent (Variables|/Script/Engine.Character|GetMesh (Variables|Default|GetPlayer%20Ref)) "HandGrip_R" "SnapToTarget" "SnapToTarget" "SnapToTarget" true)
      (Rendering|SetVisibility (Variables|Default|GetBowMesh) true true)
      (Animation|Montage|PlayMontage (Variables|/Script/Engine.Character|GetMesh (Variables|Default|GetPlayer%20Ref)) "/Game/Blueprints/Inventory/Items/Weapons/Unsheath_Sword_Anim_Montage.Unsheath_Sword_Anim_Montage" 1.0 0.0 "None" false))
    (:B
      (Rendering|SetVisibility (Variables|Default|GetBowMesh) true true)
      (Animation|Montage|PlayMontage (Variables|/Script/Engine.Character|GetMesh (Variables|Default|GetPlayer%20Ref)) "/Game/Blueprints/Inventory/Items/Weapons/Sheath_Sword_Anim_Montage.Sheath_Sword_Anim_Montage" 1.0 0.0 "None" false
        (:OnCompleted
          (Variables|/Game/Characters/FirstPerson/Blueprints/BP_ALTLI_Char.BP_ALTLI_Char_C|SetisHoldingItemRight (Variables|Default|GetPlayer%20Ref) false)
          (Variables|/Game/Characters/FirstPerson/Blueprints/BP_ALTLI_Char.BP_ALTLI_Char_C|SetHeldItemRight (Variables|Default|GetPlayer%20Ref) 0)
          (Actor|DestroyActor))))))

(fn ConstructionScript)

(fn CalculateArrowSpawnTransform
  (params (Target%20Position :type Vector))
  (bind _arrowspawn (Variables|Default|GetArrowSpawn))
  (bind _returnvalue (Transformation|GetWorldLocation _arrowspawn))
  (bind _returnvalue_2 (Math|Rotator|FindLookatRotation _returnvalue Target%20Position))
  (bind _returnvalue_3 (Math|Vector|GetForwardVector _returnvalue_2))
  (bind _returnvalue_4 (* _returnvalue_3 1e+01))
  (bind _returnvalue_5 (+ _returnvalue _returnvalue_4))
  (return (Math|Transform|MakeTransform _returnvalue_5 (Math|Rotator|FindLookatRotation _returnvalue_5 Target%20Position))))

(fn GetWeaponTarget
  (bind _returnvalue (Game|GetPlayerCameraManager 0))
  (bind _transformcomponent (Variables|/Script/Engine.PlayerCameraManager|GetTransformComponent _returnvalue))
  (bind _returnvalue_2 (Transformation|GetWorldLocation _transformcomponent))
  (bind _outhit (Collision|LineTraceByChannel _returnvalue_2 (+ _returnvalue_2 (* (Transformation|GetActorForwardVector _returnvalue) 1e+04)) "TraceTypeQuery1" false 0 "Persistent"))
  (return (Math|Vector|SelectVector (.ImpactPoint (Collision|BreakHitResult _outhit)) (.TraceEnd (Collision|BreakHitResult _outhit)) (.bBlockingHit (Collision|BreakHitResult _outhit)))))

(fn Interactwith
  (params (PlayerC :type BP%20ALTLI%20Char%20Object%20Reference))
  (return "" 0))

(fn Lookat
  (bind _itemdatacomponent (Variables|Default|GetItemDataComponent))
  (bind _itemid (Variables|/Game/Blueprints/Inventory/ItemDataComponent.ItemDataComponent_C|GetItemID _itemdatacomponent))
  (bind _returnvalue (Utilities|GetDataTableRow (.datatable _itemid) (.rowname _itemid))
    (:then
      (return (Utilities|Text|FormatText "To pick up: {item}  
press E" (.Name (Utilities|Struct|BreakFItemStruct _returnvalue)))))))

(fn RightHand?
  (return true))