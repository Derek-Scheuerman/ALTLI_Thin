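; Bow actions component that equips the player with a bow and routes input to it.
; On BeginPlay it asks the player character to add BP_Bow; its own AddWeaponOfClass event spawns, activates and stores a weapon as CurrentBow.
; Primary input sends triggered or, on cancel, released messages to CurrentBow, and secondary input sends triggered.
; A separate event snaps a weapon to the player actor, and debug prints remain throughout.
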(event Input|EnhancedActionEvents|EnhancedInputActionIA_Primary
  (params (ActionValue :type Boolean) (ElapsedSeconds :type Float%20%28double-precision%29) (TriggeredSeconds :type Float%20%28double-precision%29) (InputAction :type Input%20Action%20Object%20Reference :default "/Game/Characters/FirstPerson/Input/Actions/IA_Primary.IA_Primary"))
  (:Triggered
    (bind _asbp_bow (Utilities|Casting|CastToBP_Bow (Variables|Default|GetCurrentBow))
      (:then
        (Class|BPIWeaponInteract|Primary(Message) _asbp_bow true false false)
        (Development|PrintString "Test"))
      (:CastFailed
        (Development|PrintString "Can't Make it!"))))
  (:Canceled
    (bind _asbp_bow_2 (Utilities|Casting|CastToBP_Bow (Variables|Default|GetCurrentBow)))
    (Class|BPIWeaponInteract|Primary(Message) _asbp_bow_2 false false true)
    (Development|PrintString "Test2")))

(event Input|EnhancedActionEvents|EnhancedInputActionIA_Secondary
  (params (ActionValue :type Boolean) (ElapsedSeconds :type Float%20%28double-precision%29) (TriggeredSeconds :type Float%20%28double-precision%29) (InputAction :type Input%20Action%20Object%20Reference :default "/Game/Characters/FirstPerson/Input/Actions/IA_Secondary.IA_Secondary"))
  (Class|BPIWeaponInteract|Secondary(Message) (Variables|Default|GetCurrentBow) true false false))

(event EventBeginPlay
  (bind _asbp_altli_char (Utilities|Casting|CastToBP_ALTLI_Char (Game|GetPlayerCharacter 0)))
  (Default|AddWeaponOfClass _asbp_altli_char "/Game/Blueprints/Inventory/Items/Weapons/Bow_and_Friends/BP_Bow.BP_Bow_C")
  (Development|PrintString "Test5"))

(event EventTick
  (params (DeltaSeconds :type Float%20%28single-precision%29)))

(event EventAttachWeapontoMesh
  (params (Weapon :type BP%20Bow%20Object%20Reference) (First%20Person :type Static%20Mesh%20Component%20Object%20Reference) (Second%20Person :type Static%20Mesh%20Component%20Object%20Reference))
  (Transformation|AttachActorToActor Weapon (Game|GetPlayerCharacter 0) "None" "SnapToTarget" "SnapToTarget" "SnapToTarget" true))

(event EventAddWeaponOfClass
  (params (Bow :type BP%20Bow%20Class%20Reference))
  (bind _returnvalue (Game|GetPlayerCharacter 0))
  (bind _returnvalue_2 (Game|SpawnActorfromClass Bow (Transformation|GetActorTransform (Game|GetPlayerCharacter 0)) "Undefined" "MultiplyWithRoot" _returnvalue _returnvalue))
  (Development|PrintString "Hello")
  (Default|ActivateWeapon _returnvalue_2)
  (bind _output_get (Variables|Default|SetCurrentBow _returnvalue_2))
  (Development|PrintString (Utilities|GetDisplayName _output_get)))