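; BP_Arrow is an arrow projectile that damages characters and pushes physics objects on impact.
; It ignores its owner when moving; its first hit disables capsule collision, calls ProcessHit and destroys the actor after a delay.
; ProcessHit applies damage to Characters and an impulse to simulating components, though the impulse call has its vectors swapped, passing hit location as impulse and scaled direction as location.
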(event Custom|Process%20Hit
  (params (Hit%20Actor :type Actor%20Object%20Reference) (Hit%20Component :type Primitive%20Component%20Object%20Reference) (Hit%20Location :type Vector) (Hit%20Direction :type Vector))
  (Utilities|FlowControl|Sequence
    (:then_0
      ;[0.15 0.15 0.15 0.5] Do Damage to Any Actors that Can Be Hit
      (bind _ascharacter (Utilities|Casting|CastToCharacter Hit%20Actor))
      (Game|Damage|ApplyDamage _ascharacter (Variables|Default|GetDamage) 0 self))
    (:then_1
      ;[0.15 0.15 0.15 0.5] Add an Impulse to Any Physics Objects
      (if (Physics|IsSimulatingPhysics Hit%20Component "None")
        (Physics|AddImpulseatLocation Hit%20Component Hit%20Location (* Hit%20Direction (Variables|Default|GetPhysics%20Force)) "None")))))

(event Collision|EventActorBeginOverlap
  (params (OtherActor :type Actor%20Object%20Reference)))

(event EventTick
  (params (DeltaSeconds :type Float%20%28single-precision%29)))

(event Collision|EventHit
  (params (MyComp :type Primitive%20Component%20Object%20Reference) (Other :type Actor%20Object%20Reference) (OtherComp :type Primitive%20Component%20Object%20Reference) (bSelfMoved :type Boolean) (HitLocation :type Vector :default "0, 0, 0") (HitNormal :type Vector :default "0, 0, 0") (NormalImpulse :type Vector :default "0, 0, 0") (Hit :type Hit%20Result%20Structure%20%28by%20ref%29))
  (bind (_bblockinghit _binitialoverlap _time _distance _location _impactpoint _normal _impactnormal _physmat _hitactor _hitcomponent) (Collision|BreakHitResult Hit))
  (Utilities|FlowControl|DoOnce false
    (:Completed
      (Utilities|FlowControl|Sequence
        (:then_0
          (Collision|SetCollisionEnabled (Variables|Default|GetCapsule%20Collision) "NoCollision"))
        (:then_1
          (CallFunction|ProcessHit _hitactor _hitcomponent _impactpoint (Math|Vector|NegateVector _normal)))
        (:then_2
          ;[0.15 0.15 0.15 0.5] Destroy Actor after a while
          (Utilities|FlowControl|Delay (Variables|Default|GetDestruction%20Time))
          (Actor|DestroyActor))))))

(event EventBeginPlay
  (Collision|IgnoreActorwhenMoving (Variables|Default|GetCapsule%20Collision) (Components|GetOwner) true))

(fn ConstructionScript)