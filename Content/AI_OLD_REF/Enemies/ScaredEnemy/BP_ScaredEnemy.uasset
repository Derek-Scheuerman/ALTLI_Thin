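; Scared enemy character that exposes aggro, walk speed and patrol hooks, and can be killed by damage.
; Aggro events set a flag and swap a mesh material to red or back.
; GetPatrolPointLocation steps along a PatrolRoute spline, reversing at either end to ping-pong.
; At zero health it ragdolls with a radial impulse centred below the shot direction vector (used as a position), then destroys itself after a delay.
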(event Custom|GetAggroed
  (Rendering|Material|SetMaterial (Variables|Character|GetMesh) 1 "/AnimationSharing/AnimSharingRed.AnimSharingRed")
  (Variables|Default|SetAggroed true))

(event Custom|LoseAggro
  (Rendering|Material|SetMaterial (Variables|Character|GetMesh) 1 (Variables|Default|GetOriginalMat))
  (Variables|Default|SetAggroed false))

(event Custom|Set%20Walk%20Speed
  (params (Speed :type Float%20%28double-precision%29))
  (Variables|/Script/Engine.CharacterMovementComponent|SetMaxWalkSpeed (Variables|Character|GetCharacterMovement) Speed))

(event Custom|RagDoll
  (params (Origin :type Vector))
  (bind _mesh (Variables|Character|GetMesh))
  (Physics|SetSimulatePhysics _mesh true)
  (Physics|AddRadialImpulse _mesh (+ Origin "0.000000,0.000000,-100.000000") 3e+02 2e+04 "RIF_Constant" false)
  (Pawn|Components|CharacterMovement|DisableMovement (Variables|Character|GetCharacterMovement))
  (Collision|SetCollisionEnabled (Variables|Collision|GetCapsuleComponent) "NoCollision")
  (Utilities|FlowControl|Delay 1e+01)
  (Actor|DestroyActor))

(event EventBeginPlay
  (Variables|Default|SetOriginalMat (Rendering|Material|GetMaterial (Variables|Character|GetMesh) 1)))

(event Game|Damage|EventPointDamage
  (params (Damage :type Float%20%28single-precision%29) (DamageType :type Damage%20Type%20Object%20Reference) (HitLocation :type Vector :default "0, 0, 0") (HitNormal :type Vector :default "0, 0, 0") (HitComponent :type Primitive%20Component%20Object%20Reference) (BoneName :type Name :default "None") (ShotFromDirection :type Vector :default "0, 0, 0") (InstigatedBy :type Controller%20Object%20Reference) (DamageCauser :type Actor%20Object%20Reference) (HitInfo :type Hit%20Result%20Structure%20%28by%20ref%29))
  (bind _output_get (Variables|Default|SetHealth (- (Variables|Default|GetHealth) Damage)))
  (if (<= _output_get 0.0)
    (CallFunction|RagDoll ShotFromDirection)))

(fn ConstructionScript)

(fn GetPatrolPointLocation
  (Utilities|IsValid (Variables|PatrolRoute|GetPatrolRoute)
    (:Is%20Valid
      (Variables|PatrolRoute|SetPatrol%20Index (+ (Variables|PatrolRoute|GetPatrol%20Index) (Math|Integer|SelectInt 1 -1 (Variables|PatrolRoute|GetDirection))))
      (if (or (>= (Variables|PatrolRoute|GetPatrol%20Index) (- (Spline|GetNumberOfSplinePoints (Variables|/Game/AI_OLD_REF/Enemies/BP_PatrolRoute.BP_PatrolRoute_C|GetSpline (Variables|PatrolRoute|GetPatrolRoute))) 1)) (<= (Variables|PatrolRoute|GetPatrol%20Index) 0))
        (Variables|PatrolRoute|SetDirection (not (Variables|PatrolRoute|GetDirection))))
      (return (Spline|GetLocationatSplinePoint (Variables|/Game/AI_OLD_REF/Enemies/BP_PatrolRoute.BP_PatrolRoute_C|GetSpline (Variables|PatrolRoute|GetPatrolRoute)) (Variables|PatrolRoute|GetPatrol%20Index) "World")))))