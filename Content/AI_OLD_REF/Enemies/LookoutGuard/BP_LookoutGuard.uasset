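; BP_LookoutGuard is a lookout enemy that can alert nearby enemies to the player's location.
; Its Alert event sphere-overlaps a wide radius, collects unique AI controllers implementing BPI_Enemy and sends each a PlayerSeenMessage.
; Aggro events set a flag and swap a mesh material, restoring the original when aggro is lost.
; Point damage reduces health with debug prints; death triggers an impulse-driven ragdoll, disables movement and capsule collision, then destroys the actor after a delay.
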(event Custom|Alert
  (params (PlayerLocation :type Vector))
  (Utilities|Array|Clear (Variables|Default|GetEnemiesToAlert))
  (bind _outactors (Collision|SphereOverlapActors (Transformation|GetActorLocation self) 1e+04 (Variables|Default|GetObject%20Types) 0))
  (for _array_element _outactors
    (if (Utilities|DoesObjectImplementInterface (AI|GetAIController _array_element) "/Game/AI_OLD_REF/Enemies/BPI_Enemy.BPI_Enemy_C")
      (Utilities|Array|AddUnique (Variables|Default|GetEnemiesToAlert) (AI|GetAIController _array_element))))
  (for _array_element_2 (Variables|Default|GetEnemiesToAlert)
    (Class|BPIEnemy|PlayerSeen(Message) _array_element_2 PlayerLocation)))

(event Custom|GetAggroed
  (Rendering|Material|SetMaterial (Variables|Character|GetMesh) 1 0)
  (Variables|Default|SetAggroed true))

(event Custom|LoseAggro
  (Rendering|Material|SetMaterial (Variables|Character|GetMesh) 1 (Variables|Default|GetOriginalMat))
  (Variables|Default|SetAggroed false))

(event Custom|RagDoll
  (params (Origin :type Vector))
  (bind _mesh (Variables|Character|GetMesh))
  (Physics|SetSimulatePhysics _mesh true)
  (Physics|AddRadialImpulse _mesh (+ Origin "0.000000,0.000000,-100.000000") 3e+02 1e+05 "RIF_Constant" false)
  (Pawn|Components|CharacterMovement|DisableMovement (Variables|Character|GetCharacterMovement))
  (Collision|SetCollisionEnabled (Variables|Collision|GetCapsuleComponent) "NoCollision")
  (Utilities|FlowControl|Delay 1e+01)
  (Actor|DestroyActor))

(event EventBeginPlay
  (Variables|Default|SetOriginalMat (Rendering|Material|GetMaterial (Variables|Character|GetMesh) 1)))

(event Game|Damage|EventPointDamage
  (params (Damage :type Float%20%28single-precision%29) (DamageType :type Damage%20Type%20Object%20Reference) (HitLocation :type Vector :default "0, 0, 0") (HitNormal :type Vector :default "0, 0, 0") (HitComponent :type Primitive%20Component%20Object%20Reference) (BoneName :type Name :default "None") (ShotFromDirection :type Vector :default "0, 0, 0") (InstigatedBy :type Controller%20Object%20Reference) (DamageCauser :type Actor%20Object%20Reference) (HitInfo :type Hit%20Result%20Structure%20%28by%20ref%29))
  (Development|PrintText (Utilities|Text|FormatText "{Instigator} hit me for {damage} damage!" InstigatedBy Damage))
  (bind _output_get (Variables|Default|SetHealth (- (Variables|Default|GetHealth) Damage)))
  (if (<= _output_get 0.0)
    (Development|PrintString "Im dead")
    (CallFunction|RagDoll ShotFromDirection)))

(fn ConstructionScript)