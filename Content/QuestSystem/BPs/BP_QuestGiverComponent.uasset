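; Quest giver component that lets an NPC offer a data-table quest and give rewards when the player interacts with it.
; InteractWith checks the player's quest log, then either auto-accepts a new quest or shows W_QuestGiver.
; For a completed quest not yet turned in, it shows W_QuestRewards; showing either widget also returns the owner's name.
; DisplayQuest reads the table from QuestData, while the other lookups use DT_QuestData directly.
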(event EventBeginPlay)

(event EventTick
  (params (DeltaSeconds :type Float%20%28single-precision%29)))

(fn DisplayQuest
  (bind _questdata (Variables|Default|GetQuestData))
  ;[0.02224 0.15 0.02685 0.5] Checks quests and adds widget to the screen.
  (bind _returnvalue (Utilities|GetDataTableRow (.datatable _questdata) (.rowname _questdata))
    (:then
      (bind _returnvalue_2 (UserInterface|CreateWidget "/Game/QuestSystem/Widgets/W_QuestGiver.W_QuestGiver_C" 0 _returnvalue (.rowname _questdata)))
      (UserInterface|Viewport|AddtoViewport _returnvalue_2 0))))

(fn DisplayRewards
  (bind _questdata (Variables|Default|GetQuestData))
  (bind _returnvalue (Utilities|GetDataTableRow "/Game/QuestSystem/DataTables/DT_QuestData.DT_QuestData" (.rowname _questdata))
    (:then
      (bind _returnvalue_2 (UserInterface|CreateWidget "/Game/QuestSystem/Widgets/W_QuestRewards.W_QuestRewards_C" 0 _returnvalue (.rowname _questdata)))
      (UserInterface|Viewport|AddtoViewport _returnvalue_2 0))))

(fn Interactwith
  (bind _myplayercharacter (CallFunction|GetMyPlayerCharacter))
  (bind _returnvalue (Components|GetOwner))
  (bind _returnvalue_2 (Game|GetPlayerCharacter 0))
  (bind _questdata (Variables|Default|GetQuestData))
  (bind _returnvalue_3 (Actor|GetComponentbyClass _returnvalue_2 "/Game/QuestSystem/BPs/AC_QuestLogComponent.AC_QuestLogComponent_C"))
  (bind _returnvalue_4 (Utilities|GetDisplayName _returnvalue))
  (bind _ac_questlogcomponent (Variables|/Game/Characters/FirstPerson/Blueprints/BP_ALTLI_Char.BP_ALTLI_Char_C|GetAC_QuestLogComponent _myplayercharacter))
  ;[0.03429 0.15 0.03887 0.5] Checks to see if we already have a quest active. If not, we display quest. This allows the NPC to display quests and give rewards.
  (if (and (not (Default|QueryActiveQuest _ac_questlogcomponent (.rowname _questdata))) (not (.ReturnValue (Default|QueryCompletedQuest _ac_questlogcomponent (.rowname _questdata)))))
    (bind _returnvalue_5 (Utilities|GetDataTableRow "/Game/QuestSystem/DataTables/DT_QuestData.DT_QuestData" (.rowname (Variables|Default|GetQuestData)))
      (:then
        (if (.AutoAccept (Utilities|Struct|BreakS_QuestDetails _returnvalue_5))
          (Utilities|IsValid _returnvalue_3
            (:Is%20Valid
              (Default|AddNewQuest _returnvalue_3 (.rowname (Variables|Default|GetQuestData)))))
          (else
            (CallFunction|DisplayQuest)
            (return _returnvalue_4)))))
    (else
      (bind _array_element (Default|GetQuestActor (Variables|/Game/Characters/FirstPerson/Blueprints/BP_ALTLI_Char.BP_ALTLI_Char_C|GetAC_QuestLogComponent (CallFunction|GetMyPlayerCharacter)) (.rowname (Variables|Default|GetQuestData))))
      (if (and (Variables|/Game/QuestSystem/BPs/BP_QuestBase.BP_QuestBase_C|GetIsCompleted _array_element) (not (Variables|/Game/QuestSystem/BPs/BP_QuestBase.BP_QuestBase_C|GetIsTurnedIn _array_element)))
        (CallFunction|DisplayRewards)
        (return _returnvalue_4)))))