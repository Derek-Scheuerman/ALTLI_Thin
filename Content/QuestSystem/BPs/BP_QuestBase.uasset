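; Base quest Blueprint that tracks one quest's objective progress through its stages.
; It loads stage data from DT_QuestData by QuestID and, on BeginPlay, binds to the player's objective-ID event and seeds one objective type from inventory counts.
; Heard IDs update a progress map, with negative values lowering counts.
; Completed objectives show a notification, finished stages load the next, and the last marks completion, optionally auto-turning in through AC_QuestLogComponent.
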(event EventBeginPlay
  (CallFunction|GetQuestDetails)
  (EventDispatchers|BindEventtoOnObjectiveIDCalled (CallFunction|GetMyPlayerCharacter) (EventDispatchers|CreateEvent :!event OnObjectiveIDHeard))
  (for _array_element (.Objectives (Utilities|Struct|BreakS_StageDetails (Variables|Default|GetCurrentStageDetails)))
    (if (Utilities|Enum|Equal(Enum) (.Type (Utilities|Struct|BreakS_ObjectiveDetails _array_element)) "NewEnumerator3")
      (CallFunction|OnObjectiveIDHeard (.ObjectiveID (Utilities|Struct|BreakS_ObjectiveDetails _array_element)) (.QuantityFound (Default|QueryInventory (Variables|/Game/Characters/FirstPerson/Blueprints/BP_ALTLI_Char.BP_ALTLI_Char_C|GetAC_InventorySystem (CallFunction|GetMyPlayerCharacter)) (Utilities|String|StringToName (.ObjectiveID (Utilities|Struct|BreakS_ObjectiveDetails _array_element))) (.Quantity (Utilities|Struct|BreakS_ObjectiveDetails _array_element)))))))
  (Utilities|FlowControl|Delay 1.0)
  (bind _return (CallFunction|AreObjectivesComplete))
  (Variables|Default|SetIsCompleted _return))

(fn ConstructionScript)

(fn OnObjectiveIDHeard
  (params (ObjectiveID :type String) (Value :type Integer))
  (bind _currentobjectiveprogress (Variables|Default|GetCurrentObjectiveProgress))
  (bind (_value _returnvalue) (Utilities|Map|Find _currentobjectiveprogress ObjectiveID))
  ;[0.0243 0.15 0.03388 0.5] When it hears the objective, it is going to check current objective progress to look for a match. If there is a match it will add a one to it. Otherwise, it will just return out. This also includes the value for inventory. If the player drops a quest item from their inventory, then the quest will read incomplete until the player picks up the item.
  (if (> (Class|KismetMathLibrary|SignOfInteger Value) 0)
    (if _returnvalue
      (if (< _value (Utilities|Struct|BreakS_ObjectiveDetails (CallFunction|GetObjectiveDatabyID ObjectiveID)))
        (Utilities|Map|Add (Variables|Default|GetCurrentObjectiveProgress) ObjectiveID (+ _value Value))
        (CallFunction|IsObjectiveComplete ObjectiveID)
        (Default|CallOnObjectiveHeard)
        (return))
      (else
        (return)))
    (else
      (Utilities|Map|Add (Variables|Default|GetCurrentObjectiveProgress) ObjectiveID (+ (.Value (Utilities|Map|Find (Variables|Default|GetCurrentObjectiveProgress) ObjectiveID)) Value))
      (return))))

(fn GetQuestDetails
  (bind _returnvalue (Utilities|GetDataTableRow "/Game/QuestSystem/DataTables/DT_QuestData.DT_QuestData" (Variables|Default|GetQuestID))
    (:then
      (bind _output_get (Variables|Default|SetQuestDetails _returnvalue))
      (bind _output_get_2 (Variables|Default|SetCurrentStageDetails (Utilities|Array|Get(acopy) (.Stages (Utilities|Struct|BreakS_QuestDetails _output_get)) (Variables|Default|GetCurrentStage))))
      (Utilities|Map|Clear (Variables|Default|GetCurrentObjectiveProgress))
      (for _array_element (.Objectives (Utilities|Struct|BreakS_StageDetails _output_get_2))
        (Utilities|Map|Add (Variables|Default|GetCurrentObjectiveProgress) (.ObjectiveID (Utilities|Struct|BreakS_ObjectiveDetails _array_element)) 0)))))

(fn GetObjectiveDatabyID
  (params (ObjectiveID :type String))
  (for _array_element (.Objectives (Utilities|Struct|BreakS_StageDetails (Variables|Default|GetCurrentStageDetails)))
    (if (Utilities|Enum|Equal(Enum) (.ObjectiveID (Utilities|Struct|BreakS_ObjectiveDetails _array_element)) ObjectiveID)
      (return _array_element))))

(fn IsObjectiveComplete
  (params (ObjectiveID :type String))
  (bind _array_element (CallFunction|GetObjectiveDatabyID ObjectiveID))
  (bind (_description _quantity) (Utilities|Struct|BreakS_ObjectiveDetails _array_element))
  ;[0.01882 0.15 0.02602 0.5] Had objective been completed? If so, then add it to the viewport, while checking all objectives.
  (if (>= (.Value (Utilities|Map|Find (Variables|Default|GetCurrentObjectiveProgress) ObjectiveID)) _quantity)
    (bind _returnvalue (UserInterface|CreateWidget "/Game/QuestSystem/Widgets/W_QuestNotification.W_QuestNotification_C" 0 _description))
    (UserInterface|Viewport|AddtoViewport _returnvalue 0)
    (bind _return (CallFunction|AreObjectivesComplete))
    (if _return
      (bind _result (Math|Integer|IncrementInt (Variables|Default|GetCurrentStage))
        (:%20%20
          (if (Utilities|Array|IsValidIndex (.stages (Variables|Default|GetQuestDetails)) _result)
            (CallFunction|GetQuestDetails)
            (else
              (Variables|Default|SetIsCompleted true)
              (if (.autocomplete (Variables|Default|GetQuestDetails))
                (Default|TurninQuest (Actor|GetComponentbyClass (Game|GetPlayerCharacter 0) "/Game/QuestSystem/BPs/AC_QuestLogComponent.AC_QuestLogComponent_C") (Variables|Default|GetQuestID))))))))))

(fn AreObjectivesComplete
  ;[0.02409 0.15 0.03207 0.5] This is going to go through each objectives to check if they are complete. If they are complete, nothing will happen. If they are not complete, then we stop this process.
  (for _array_element (.Objectives (Utilities|Struct|BreakS_StageDetails (Variables|Default|GetCurrentStageDetails)))
    (if (not (>= (.Value (Utilities|Map|Find (Variables|Default|GetCurrentObjectiveProgress) (.ObjectiveID (Utilities|Struct|BreakS_ObjectiveDetails _array_element)))) (.Quantity (Utilities|Struct|BreakS_ObjectiveDetails (CallFunction|GetObjectiveDatabyID (.ObjectiveID (Utilities|Struct|BreakS_ObjectiveDetails _array_element)))))))
      (bind _output_get (LocalVariables|SetLocal_AllComplete false))
      (return _output_get)))
  (return (LocalVariables|GetLocal_AllComplete)))